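; BP_PC is a player controller that sets up the local player's UI and input and relays light intensity change requests.
; On BeginPlay, the local controller adds WBP_UserWidget to the viewport, shows the cursor, adds the default Enhanced Input context and sets game-only input.
; Its Server_RequestChangeLight event finds a BP_Light in the level and calls MCChangeLight, a server-to-multicast pattern judging by the names.
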(event Custom|Server_RequestChangeLight
  (params (NewIntensity :type Float%20%28single-precision%29))
  (bind _returnvalue (Actor|GetActorOfClass "/Game/MyProject/Blueprint/Object/BP_Light.BP_Light_C"))
  (Default|MCChangeLight _returnvalue NewIntensity))

(event EventBeginPlay
  (if (Pawn|IsLocalPlayerController)
    (bind _returnvalue (UserInterface|CreateWidget "/Game/MyProject/Blueprint/UI/WBP_UserWidget.WBP_UserWidget_C"))
    (UserInterface|Viewport|AddtoViewport _returnvalue 0)
    (Variables|Default|SetbShowMouseCursor true)
    (Input|AddMappingContext (PlayerController|LocalPlayerSubsystems|GetEnhancedInputLocalPlayerSubsystem) "/Game/MyProject/Input/IMC_Default.IMC_Default" 0 "(bIgnoreAllPressedKeysUntilRelease=True,bForceImmediately=False,bNotifyUserSettings=False)")
    (Input|SetInputModeGameOnly (Game|GetPlayerController 0) false)))

(fn ConstructionScript)