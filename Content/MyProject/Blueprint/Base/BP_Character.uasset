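; Player character base that handles move, look and jump input and leaves flowers at its feet while moving.
; The shoot input only toggles a close camera view, changing spring arm length and hiding the mesh from its owner.
; Flower spawning is distance-gated, but the stored last location is built from the spacing value, not the actor's position.
; Single-axis movement direction picks the flower's orb material and gives it a short lifespan.
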(event Custom|spawnflower
  (bind _returnvalue (Transformation|GetActorLocation))
  (bind _action_value_x (Variables|Default|GetAction%20Value%20X))
  (bind _action_value_y (Variables|Default|GetAction%20Value%20Y))
  (bind _returnvalue_2 (== _action_value_y 0.0))
  (bind _returnvalue_3 (== _action_value_x 0.0))
  (if (>= (Math|Vector|Distance(Vector) (Transformation|GetActorLocation) (Variables|Default|GetLastFlowerLocation)) (Variables|Default|GetFlowerSpawnDistance))
    (bind _returnvalue_4 (Game|SpawnActorfromClass "/Game/MyProject/Blueprint/Object/BP_Flower.BP_Flower_C" (Math|Transform|MakeTransform (Math|Vector|MakeVector (.x _returnvalue) (.y _returnvalue) (- (.z _returnvalue) 9e+01)) "0, 0, 0" "1.000000,1.000000,1.000000") "Undefined" "MultiplyWithRoot" 0 0))
    (Variables|Default|SetBP_Flower _returnvalue_4)
    (Variables|Default|SetLastFlowerLocation (Math|Conversions|ToVector(Float) (Variables|Default|GetFlowerSpawnDistance)))
    (Utilities|FlowControl|Sequence
      (:then_0
        (if (and (> (Variables|Default|GetAction%20Value%20X) 0.0) _returnvalue_2)
          (for (_array_element _array_index) (Variables|/Script/Exhibition.Flower|GetLightOrbs (Variables|Default|GetBP_Flower))
            (Rendering|Material|SetMaterial _array_element _array_index "/Game/CR/LQ/AMT_Materials/MI_Light_4_0.MI_Light_4_0")
            (Actor|SetLifeSpan (Variables|Default|GetBP_Flower) 5.0))))
      (:then_1
        (if (and _returnvalue_2 (< (Variables|Default|GetAction%20Value%20X) 0.0))
          (for (_array_element_2 _array_index_2) (Variables|/Script/Exhibition.Flower|GetLightOrbs (Variables|Default|GetBP_Flower))
            (Rendering|Material|SetMaterial _array_element_2 _array_index_2 "/Game/CR/LQ/AMT_Materials/MI_Light_2_0.MI_Light_2_0")
            (Actor|SetLifeSpan (Variables|Default|GetBP_Flower) 5.0))))
      (:then_2
        (if (and (> (Variables|Default|GetAction%20Value%20Y) 0.0) _returnvalue_3)
          (for (_array_element_3 _array_index_3) (Variables|/Script/Exhibition.Flower|GetLightOrbs (Variables|Default|GetBP_Flower))
            (Rendering|Material|SetMaterial _array_element_3 _array_index_3 "/Game/CR/LQ/AMT_Materials/MI_Light_1_0.MI_Light_1_0")
            (Actor|SetLifeSpan (Variables|Default|GetBP_Flower) 5.0))))
      (:then_3
        (if (and _returnvalue_3 (< (Variables|Default|GetAction%20Value%20Y) 0.0))
          (for (_array_element_4 _array_index_4) (Variables|/Script/Exhibition.Flower|GetLightOrbs (Variables|Default|GetBP_Flower))
            (Rendering|Material|SetMaterial _array_element_4 _array_index_4 "/Game/CR/LQ/AMT_Materials/MI_Light_4_2.MI_Light_4_2")
            (Actor|SetLifeSpan (Variables|Default|GetBP_Flower) 5.0)))))))

(event Input|EnhancedActionEvents|EnhancedInputActionIA_Move
  (params (ActionValue :type Vector%202D%20Structure) (ElapsedSeconds :type Float%20%28double-precision%29) (TriggeredSeconds :type Float%20%28double-precision%29) (InputAction :type Input%20Action%20Object%20Reference :default "/Game/MyProject/Input/IA_Move.IA_Move"))
  (bind _output_get (Variables|Default|SetAction%20Value%20X (.x ActionValue)))
  (bind _output_get_2 (Variables|Default|SetAction%20Value%20Y (.y ActionValue)))
  (Class|MyCharacter|Move _output_get_2 _output_get)
  (CallFunction|Spawnflower))

(event Input|EnhancedActionEvents|EnhancedInputActionIA_Look
  (params (ActionValue :type Vector%202D%20Structure) (ElapsedSeconds :type Float%20%28double-precision%29) (TriggeredSeconds :type Float%20%28double-precision%29) (InputAction :type Input%20Action%20Object%20Reference :default "/Game/MyProject/Input/IA_Look.IA_Look"))
  (Class|MyCharacter|Look (* (.y ActionValue) -1.0) (.x ActionValue)))

(event Input|EnhancedActionEvents|EnhancedInputActionIA_Jump
  (params (ActionValue :type Boolean) (ElapsedSeconds :type Float%20%28double-precision%29) (TriggeredSeconds :type Float%20%28double-precision%29) (InputAction :type Input%20Action%20Object%20Reference :default "/Game/MyProject/Input/IA_Jump.IA_Jump"))
  (:Started
    (Character|Jump))
  (:Completed
    (Character|StopJumping)))

(event Input|EnhancedActionEvents|EnhancedInputActionIA_Shoot
  (params (ActionValue :type Boolean) (ElapsedSeconds :type Float%20%28double-precision%29) (TriggeredSeconds :type Float%20%28double-precision%29) (InputAction :type Input%20Action%20Object%20Reference :default "/Game/MyProject/Input/IA_Shoot.IA_Shoot"))
  (bind _springarm (Variables|Default|GetSpringArm))
  (:Started
    (bind _output_get (Variables|Default|SetIsShoot (not (Variables|Default|GetIsShoot))))
    (if _output_get
      (Variables|/Script/Engine.SpringArmComponent|SetTargetArmLength _springarm -55.0)
      (Class|PrimitiveComponent|SetOwnerNoSee (Variables|Character|GetMesh) true)
      (else
        (Variables|/Script/Engine.SpringArmComponent|SetTargetArmLength _springarm 2e+02)
        (Class|PrimitiveComponent|SetOwnerNoSee (Variables|Character|GetMesh) false)))))

(fn ConstructionScript)